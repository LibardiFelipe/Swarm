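; Menu player controller that shows the main menu and handles hosting and joining multiplayer sessions.
; On BeginPlay, the local controller creates the main menu widget and adds it to the viewport.
; HostSession creates an Advanced Sessions session tagged with a key/value property, then opens the debug map as a listen server.
; JoinSession searches for a single session matching that property and joins it, printing Portuguese error messages on failure.
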(event `self.ReceiveBeginPlay`
  (if (`self.IsLocalController`)
    (bind _returnvalue (`|CreateWidget` "/Game/UI/Menus/MainMenuWB.MainMenuWB_C" self))
    (bind _output_get (set `self.MenuWB` _returnvalue))
    (`UserWidget.AddToViewport` _output_get 0)))

(event `HostSession`
  (`CreateSessionCallbackProxyAdvanced.CreateAdvancedSession` (`|MakeArray` (`AdvancedSessionsLibrary.MakeLiteralSessionPropertyString` (`self.KeyName`) (`self.KeyValue`))) self
    (:`OnSuccess`
      (`GameplayStatics.OpenLevel` "DebugMAP" true "listen"))))

(event `JoinSession`
  (bind _results (`FindSessionsCallbackProxyAdvanced.FindSessionsAdvanced` self 1 false "AllServers" (`|MakeArray` (`AdvancedSessionsLibrary.MakeLiteralSessionSearchProperty` (`AdvancedSessionsLibrary.MakeLiteralSessionPropertyString` (`self.KeyName`) (`self.KeyValue`)) "Equals")))
    (:`OnSuccess`
      (`JoinSessionCallbackProxy.JoinSession` self (`|GetArrayItem` _results)
        (:`OnFailure`
          (`KismetSystemLibrary.PrintString` "Falha ao conectar-se à sessão!"))))
    (:`OnFailure`
      (`KismetSystemLibrary.PrintString` "Falha ao encontrar sessões!"))))

(fn `UserConstructionScript`)