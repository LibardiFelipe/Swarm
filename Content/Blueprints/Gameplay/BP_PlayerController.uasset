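; Player controller that manages the class selector widget, showing it on BeginPlay for the local controller.
; The ClassSelector input action toggles it through SwitchClassSelector, which adds the widget to or removes it from the viewport.
; The widget is created lazily on first use and then reused, with HandleMouseCursor switched on or off alongside it.
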(event `self.ReceiveBeginPlay`
  (`|ExecutionSequence`
    (:`then_0`
      (if (`self.IsLocalController`)
        (`self.SwitchClassSelector`)))))

(event `SwitchClassSelector`
  (`/Engine/EditorBlueprintResources/StandardMacros.IsValid` (`self.ClassSelectorWB`)
    (:`Is Valid`
      (if (`Widget.IsInViewport` (`self.ClassSelectorWB`))
        (`Widget.RemoveFromParent` (`self.ClassSelectorWB`))
        (`self.HandleMouseCursor` false)
        (else
          (`UserWidget.AddToViewport` (stale _output_get) 0 :!label _label)
          (`self.HandleMouseCursor` true))))
    (:`Is Not Valid`
      (bind _returnvalue (`|CreateWidget` "/Game/UI/Gameplay/ClassSelectorWB.ClassSelectorWB_C" self))
      (bind _output_get (set `self.ClassSelectorWB` _returnvalue))
      (goto _label))))

(event `InputAction|ClassSelector`
  (params (Key :type "Key Structure"))
  (:`Pressed`
    (`self.SwitchClassSelector`)))

(fn `UserConstructionScript`)